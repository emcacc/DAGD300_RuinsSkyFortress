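; Elevator actor that the first-person character raises and lowers with key presses while standing in its trigger box.
; Box overlap enables input for player 0 on entry and disables it on exit, limited to FirstPersonCharacter.
; E plays and R reverses a timeline whose alpha lerps the Elevator component's relative location between StartLocation and EndLocation, without sweep.
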(event `Key|E`
  (params (Key :type "Key Structure"))
  (:`Pressed`
    (bind (_direction _alpha) (`Timeline|Moving Up/Down` :!label _label)
      (:`Update`
        (`SceneComponent.K2_SetRelativeLocation` (`self.Elevator`) (`KismetMathLibrary.VLerp` (`self.Start Location`) (`self.End Location`) _alpha) false false)))))

(event `Key|R`
  (params (Key :type "Key Structure"))
  (:`Pressed`
    (goto _label :!via `Reverse`)))

(event `self.Box.OnComponentBeginOverlap`
  (params (OverlappedComponent :type "PrimitiveComponent Object Reference") (OtherActor :type "Actor Object Reference") (OtherComp :type "PrimitiveComponent Object Reference") (OtherBodyIndex :type Integer) (bFromSweep :type Boolean) (SweepResult :type "HitResult Structure (by ref)"))
  ;[1 1 1] Overlay Inputs
  (cast `/Game/FirstPersonBP/Blueprints/FirstPersonCharacter` OtherActor)
  (`self.EnableInput` (`GameplayStatics.GetPlayerController` 0)))

(event `self.Box.OnComponentEndOverlap`
  (params (OverlappedComponent :type "PrimitiveComponent Object Reference") (OtherActor :type "Actor Object Reference") (OtherComp :type "PrimitiveComponent Object Reference") (OtherBodyIndex :type Integer))
  ;[1 1 1] Overlay Inputs
  (cast `/Game/FirstPersonBP/Blueprints/FirstPersonCharacter` OtherActor)
  (`self.DisableInput` (`GameplayStatics.GetPlayerController` 0)))

(fn `UserConstructionScript`)