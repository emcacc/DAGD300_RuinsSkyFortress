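; Turret enemy that turns toward and shoots at the first-person player character when its PawnSensing component sees one.
; Each sighting snaps the whole actor's rotation to face the character.
; It then spawns a FirstPersonProjectile at ProjectileSpawnLocation and launches it along TurretTop's forward vector with a velocity-change impulse scaled by ShootForce.
; A SpawnProjectile flag, reset after a short Delay, limits the fire rate.
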(event `self.PawnSensing.OnSeePawn`
  (params (Pawn :type "Pawn Object Reference"))
  (bind _asfirst_person_character (cast `/Game/FirstPersonBP/Blueprints/FirstPersonCharacter` Pawn))
  (`|ExecutionSequence`
    (:`then_0`
      (`self.K2_SetActorRotation` (`KismetMathLibrary.FindLookAtRotation` (`self.K2_GetActorLocation`) (`self.K2_GetActorLocation` _asfirst_person_character))))
    (:`then_1`
      (if (`self.Spawn_Projectile`)
        (bind _returnvalue (`|SpawnActorFromClass` "/Game/FirstPersonBP/Blueprints/FirstPersonProjectile.FirstPersonProjectile_C" (`SceneComponent.K2_GetComponentToWorld` (`self.ProjectileSpawnLocation`)) "Undefined" "OverrideRootScale" null null))
        (`PrimitiveComponent.AddImpulse` (`/Game/FirstPersonBP/Blueprints/FirstPersonProjectile.Sphere` _returnvalue) (* (`SceneComponent.GetForwardVector` (`self.Turret Top`)) (`self.Shoot_Force`)) "None" true)
        (set `self.Spawn_Projectile` false)
        (`KismetSystemLibrary.Delay` 1.5)
        (set `self.Spawn_Projectile` true)))))

(fn `UserConstructionScript`)