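; Sci-fi double sliding door that the player opens with the Use input while inside its trigger volume.
; Trigger overlap enables input for the first player controller, and end overlap disables it and reverses the door, with no check on the overlapping actor.
; The DoorOpen timeline slides the two panels apart along local X in opposite directions.
; An IsOpen toggle branch is left unconnected and never runs.
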(event `InputAction|Use`
  (params (Key :type "Key Structure"))
  (:`Pressed`
    (bind (_direction _percent) (`Timeline|DoorOpen` :!label _label)
      (:`Update`
        (bind _returnvalue (* _percent 200.0))
        (`SceneComponent.K2_SetRelativeLocation` (`self.DoorLeft`) (`KismetMathLibrary.MakeVector` _returnvalue) false false)
        (`SceneComponent.K2_SetRelativeLocation` (`self.DoorRight`) (`KismetMathLibrary.MakeVector` (* _returnvalue -1.0)) false false)))))

(event `self.TriggerVolume.OnComponentBeginOverlap`
  (params (OverlappedComponent :type "PrimitiveComponent Object Reference") (OtherActor :type "Actor Object Reference") (OtherComp :type "PrimitiveComponent Object Reference") (OtherBodyIndex :type Integer) (bFromSweep :type Boolean) (SweepResult :type "HitResult Structure (by ref)"))
  (`self.EnableInput` (`GameplayStatics.GetPlayerController` 0)))

(event `self.TriggerVolume.OnComponentEndOverlap`
  (params (OverlappedComponent :type "PrimitiveComponent Object Reference") (OtherActor :type "Actor Object Reference") (OtherComp :type "PrimitiveComponent Object Reference") (OtherBodyIndex :type Integer))
  (`self.DisableInput` (`GameplayStatics.GetPlayerController` 0))
  (goto _label :!via `Reverse`))

(fn `UserConstructionScript`)